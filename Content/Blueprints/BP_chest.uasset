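; BP_chest is an interactable chest that opens when the player holds two keys and lets a linked door open.
; Interaction reads Key1 and Key2 from BP_FirstPersonCharacter, adding a dummy key mesh for each held key on every call.
; With both keys, a DoOnce plays a Timeline that rotates the cover and sets BPDoor.CanOpen.
; Otherwise, it prints which key is missing.
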(event EventBeginPlay)

(event Collision|EventActorBeginOverlap
  (params (OtherActor :type Actor%20Object%20Reference)))

(event EventTick
  (params (DeltaSeconds :type Float%20%28single-precision%29)))

(event EventInteraction
  (bind _asbp_first_person_character (Utilities|Casting|CastToBP_FirstPersonCharacter (Game|GetPlayerCharacter 0)))
  (Utilities|FlowControl|Sequence
    (:then_0
      (if (Variables|/Game/Blueprints/Implemented/BP_FirstPersonCharacter.BP_FirstPersonCharacter_C|GetKey1 _asbp_first_person_character)
        (bind _returnvalue (AddComponent|AddStaticMeshComponent false (Math|Transform|MakeTransform "-20.000000,50.000000,55.000000" "-90.000000,0.000000,180.000000" "1.000000,1.000000,1.000000")))
        (Variables|Default|SetDummy%20Key%201 _returnvalue)))
    (:then_1
      (if (Variables|/Game/Blueprints/Implemented/BP_FirstPersonCharacter.BP_FirstPersonCharacter_C|GetKey2 _asbp_first_person_character)
        (bind _returnvalue_2 (AddComponent|AddStaticMeshComponent false (Math|Transform|MakeTransform "19.000000,50.000000,55.000000" "-90.000000,0.000000,180.000000" "1.000000,1.000000,1.000000")))
        (Variables|Default|SetDummy%20Key%202 _returnvalue_2)))
    (:then_2
      (if (Variables|/Game/Blueprints/Implemented/BP_FirstPersonCharacter.BP_FirstPersonCharacter_C|GetKey1 _asbp_first_person_character)
        (if (Variables|/Game/Blueprints/Implemented/BP_FirstPersonCharacter.BP_FirstPersonCharacter_C|GetKey2 _asbp_first_person_character)
          (Utilities|FlowControl|DoOnce false
            (:Completed
              (bind _ouverture (Timeline|Timeline Play)
                (:Update
                  (Transformation|SetRelativeRotation (Variables|Default|GetChest_cover_StaticMeshComponent0) (Math|Rotator|MakeRotator (* _ouverture (Variables|Default|GetRotation%20Angle)) 0.0 0.0) false false)
                  (Variables|/Game/Blueprints/BP_Door.BP_Door_C|SetCanOpen (Variables|Default|GetBP_Door) true)))))
          (else
            (Development|PrintString "Key 2 missing")))
        (else
          (Development|PrintString "Key 1 missing !!!"))))))

(fn ConstructionScript)