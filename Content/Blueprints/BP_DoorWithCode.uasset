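; Double door that unlocks through a three-press button code and then swings open.
; ButtonInteraction counts presses and those the caller flags as in the right order; three correct set CanOpen and trigger Interaction, otherwise both counters reset.
; Once unlocked, Interaction alternates opening and closing via a FlipFlop and a Timeline that yaws the two leaves in opposite directions, scaled by RotationAngle and SpeedOpening.
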(event Custom|ButtonInteraction
  (params (GoodOrder :type Boolean))
  (bind _result (Math|Integer|IncrementInt (Variables|Default|GetNbInput))
    (:%20%20
      (Variables|Default|SetNbInput _result)
      (if GoodOrder
        (bind _result_2 (Math|Integer|IncrementInt (Variables|Default|GetInputOrder))
          (:%20%20
            (Variables|Default|SetInputOrder _result_2))))
      (if (== (Variables|Default|GetNbInput) 3)
        (if (== (Variables|Default|GetInputOrder) 3)
          (Variables|Default|SetCanOpen true)
          (CallFunction|Interaction)
          (Development|PrintString "WELL DONE")
          (else
            (CallFunction|WrongOrder)))))))

(event Custom|WrongOrder
  (Development|PrintString "NAN")
  (Variables|Default|SetInputOrder 0)
  (Variables|Default|SetNbInput 0))

(event EventBeginPlay)

(event Collision|EventActorBeginOverlap
  (params (OtherActor :type Actor%20Object%20Reference)))

(event EventTick
  (params (DeltaSeconds :type Float%20%28single-precision%29)))

(event EventInteraction
  (if (Variables|Default|GetCanOpen)
    (Components|Timeline|SetPlayRate (Variables|Default|GetTimeline) (/ 1.0 (Variables|Default|GetSpeedOpening)))
    (Utilities|FlowControl|FlipFlop
      (:A
        (bind _newtrack_1 (Timeline|Timeline Play)
          (:Update
            (Transformation|SetRelativeRotation (Variables|Default|GetDoor_3_StaticMeshComponent0) (Math|Rotator|MakeRotator 0.0 0.0 (* (* _newtrack_1 (Variables|Default|GetRotation%20Angle)) -1.0)) false false)
            (Transformation|SetRelativeRotation (Variables|Default|GetDoor_4_StaticMeshComponent0) (Math|Rotator|MakeRotator 0.0 0.0 (* _newtrack_1 (Variables|Default|GetRotation%20Angle))) false false))))
      (:B
        (Timeline|Timeline Reverse)))
    (else
      (Development|PrintString "Nan"))))

(fn ConstructionScript)